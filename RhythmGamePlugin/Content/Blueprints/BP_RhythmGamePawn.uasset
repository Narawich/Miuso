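; Player pawn for a five-lane rhythm game that routes key input to beat players and tracks score, combo and mistakes.
; It spawns a BP_Lane at each child-actor BP_BeatPlayer from the song reader's lane data and creates the game UI.
; Hits raise score with a combo-based multiplier capped at five, while misses lower the song volume.
; Too many consecutive wrong or missed beats trigger game over through the SongReader.
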(event `CreateLanes`
  (params (songReader :type "/RhythmGamePlugin/Blueprints/BP_SongReader Object Reference") (laneData :type "Array of LaneData Structure") (sequenceLength :type "Float (double-precision)") (BPM :type "Float (double-precision)"))
  ;[1 1 1] Create lanes
  (set `self.songReader` songReader)
  (`self.CreateGameUI`)
  (`self.StoreAllBeatPlayers`)
  (for (_array_element _array_index) laneData
    (if (<= _array_index (`KismetArrayLibrary.Array_LastIndex` (`self.beatPlayers`)))
      (bind _returnvalue (`|SpawnActorFromClass` "/RhythmGamePlugin/Blueprints/BP_Lane.BP_Lane_C" (`KismetMathLibrary.Conv_VectorToTransform` (`self.K2_GetActorLocation` (`|GetArrayItem` (`self.beatPlayers`) _array_index))) "Undefined" "OverrideRootScale" null _array_element sequenceLength BPM _array_index null))
      (`/RhythmGamePlugin/Blueprints/BP_Lane.Initialize` _returnvalue)
      (`KismetArrayLibrary.Array_Add` (`self.lanes`) _returnvalue))))

(event `StoreAllBeatPlayers`
  ;[1 1 1] Initialize the beat players
  (`KismetArrayLibrary.Array_Clear` (`self.beatPlayers`))
  (for _array_element (`|MakeArray` (`self.1LaneBeatPlayer`) (`self.2LaneBeatPlayer`) (`self.3LaneBeatPlayer`) (`self.4LaneBeatPlayer`) (`self.5LaneBeatPlayer`))
    (bind _asbp_beat_player (cast `/RhythmGamePlugin/Blueprints/BP_BeatPlayer` (`ChildActorComponent.ChildActor` _array_element)))
    (`/RhythmGamePlugin/Blueprints/BP_BeatPlayer.Initialize` _asbp_beat_player self)
    (`KismetArrayLibrary.Array_Add` (`self.beatPlayers`) _asbp_beat_player)))

(event `CreateGameUI`
  ;[1 1 1] Show game UI
  (bind _returnvalue (`|CreateWidget` "/RhythmGamePlugin/Blueprints/UI/BP_GameUI.BP_GameUI_C"))
  (bind _output_get (set `self.gameUI` _returnvalue))
  (`UserWidget.AddToViewport` _output_get 0))

(event `StartGame`
  ;[1 1 1] Reset score and start the game
  (`self.ResetScore`)
  (set `self.missedBeatsInARow` 0)
  (set `self.maxCombo` 0)
  (for _array_element (`self.lanes`)
    (`/RhythmGamePlugin/Blueprints/BP_Lane.MoveTheLane` _array_element)))

(event `Key|AnyKey`
  (params (Key :type "Key Structure"))
  ;[1 1 1] Detect player input
  (:`Pressed`
    (set `self.keyPressed` true)
    (for _array_element (`self.beatPlayers`) :!label _label
      (if (== (`.Key` (break `InputActionKeyMapping` (`/RhythmGamePlugin/Blueprints/BP_BeatPlayer.key` _array_element))) Key)
        (`/RhythmGamePlugin/Blueprints/BP_BeatPlayer.KeyInput` _array_element (`self.keyPressed`)))))
  (:`Released`
    (set `self.keyPressed` false)
    (goto _label)))

(event `OnBeatPlayed`
  ;[1 1 1] On beat played successfuly
  (`SongReader.SetSongVolume` (`self.songReader`) 1.0)
  (set `self.missedBeatsInARow` 0)
  (`self.IncreaseScore` 50)
  (`self.IncreaseCombo`))

(event `OnWrongBeat`
  ;[1 1 1] On failed to play beat
  (`self.ResetCombo` :!label _label_2)
  (bind _result (`/Engine/EditorBlueprintResources/StandardMacros.IncrementInt` (`self.missedBeatsInARow`))
    (:`  `
      (if (and (>= _result (`self.mistakesInARowToGameOver`)) (not (`/RhythmGamePlugin/Blueprints/BP_SongReader.isGameOver` (`self.songReader`))))
        (`/RhythmGamePlugin/Blueprints/BP_SongReader.GameOver` (`self.songReader`))))))

(event `OnBeatMissed`
  ;[1 1 1] On failed to play beat
  (`SongReader.SetSongVolume` (`self.songReader`) 0.25)
  (goto _label_2))

(event `OnGameOver`
  ;[1 1 1] Destory lanes on game over
  (`Widget.RemoveFromParent` (`self.gameUI`))
  (bind (_arrayindex _arrayelement) (`/Engine/EditorBlueprintResources/StandardMacros.ReverseForEachLoop` (`self.lanes`))
    (:`LoopBody`
      (`/Engine/EditorBlueprintResources/StandardMacros.IsValid` _arrayelement
        (:`Is Valid`
          (`self.K2_DestroyActor` _arrayelement))))))

(event `IncreaseScore`
  (params (scoreToAdd :type Integer))
  ;[1 1 1] Score calculation
  (bind _output_get (set `self.score` (+ (`self.score`) (* scoreToAdd (`self.scoreMultiplier`)))))
  (`/RhythmGamePlugin/Blueprints/UI/BP_GameUI.UpdateScore` (`self.gameUI`) _output_get))

(event `IncreaseCombo`
  ;[1 1 1] Score calculation
  (bind _result (`/Engine/EditorBlueprintResources/StandardMacros.IncrementInt` (`self.combo`))
    (:`  `
      (`/RhythmGamePlugin/Blueprints/UI/BP_GameUI.UpdateCombo` (`self.gameUI`) _result)
      (`self.CalculateMultiplier`)
      (set `self.maxCombo` (`KismetMathLibrary.Max` (`self.combo`) (`self.maxCombo`))))))

(event `ResetCombo`
  ;[1 1 1] Score calculation
  (bind _output_get (set `self.combo` 0))
  (`/RhythmGamePlugin/Blueprints/UI/BP_GameUI.UpdateCombo` (`self.gameUI`) _output_get)
  (`self.CalculateMultiplier`))

(event `CalculateMultiplier`
  ;[1 1 1] Score calculation
  (bind _output_get (set `self.scoreMultiplier` (`KismetMathLibrary.Clamp` (+ (`.ReturnValue` (`KismetMathLibrary.FMod` (`KismetMathLibrary.Conv_IntToDouble` (`self.combo`)) 10.0)) 1) 1 5)))
  (`/RhythmGamePlugin/Blueprints/UI/BP_GameUI.UpdateMultiplier` (`self.gameUI`) _output_get)
  (`self.CalculateComboCounter`))

(event `ResetScore`
  ;[1 1 1] Score calculation
  (bind _output_get (set `self.score` 0))
  (`/RhythmGamePlugin/Blueprints/UI/BP_GameUI.UpdateScore` (`self.gameUI`) _output_get)
  (set `self.scoreMultiplier` 1)
  (`self.ResetCombo`))

(event `CalculateComboCounter`
  (bind _gameui (`self.gameUI`))
  (bind (_remainder _returnvalue) (`KismetMathLibrary.FMod` (`KismetMathLibrary.Conv_IntToDouble` (`self.combo`)) 10.0))
  ;[1 1 1] Score calculation
  (if (or (!= _remainder 0.0) (== _returnvalue 0))
    (`/RhythmGamePlugin/Blueprints/UI/BP_GameUI.UpdateComboCounter` _gameui _remainder)
    (else
      (`/RhythmGamePlugin/Blueprints/UI/BP_GameUI.UpdateComboCounter` _gameui 10.0))))

(fn `UserConstructionScript`)